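; AngieCueBP is a base cue for the monster Angie that fires when she enters it, with children adding more specific behavior.
; AngieEnters stores the actor, optionally sets her AI controller to waiting, marks the cue triggered and optionally plays a conversation sound.
; Once triggered, Tick counts down the wait duration and flags the cue finished, without releasing Angie here.
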(event `self.ReceiveBeginPlay`)

(event `self.ReceiveActorBeginOverlap`
  (params (OtherActor :type "Actor Object Reference")))

(event `self.ReceiveTick`
  (params (DeltaSeconds :type "Float (single-precision)"))
  (if (`self.triggered`)
    (bind _output_get (set `self.WaitDuration` (- (`self.WaitDuration`) DeltaSeconds)))
    (if (< _output_get 0.0)
      (set `self.finished` true))))

(fn `AngieEnters`
  (params (angieActor :type "/Game/Monsters/AI/Angie/Angie Object Reference"))
  ;[1 1 1] Children will add more specific behavior
  (bind _output_get (set `self.angie` angieActor))
  (if (`self.StopsAngie`)
    (`/Game/Monsters/AI/Angie/AngieController.SetWaiting` (`/Game/Monsters/AI/Angie/Angie.aicontroller` _output_get) true))
  (set `self.triggered` true)
  (if (`self.HasSound`)
    (`/Game/Sound_Assets/Voice/Conversation.Play` (`self.Conversation`))))

(fn `UserConstructionScript`)