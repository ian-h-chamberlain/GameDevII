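; Story trigger that cues Angie when she or the player (Derek) overlaps it at a StoryIndex matching the BlockingSmoke's.
; It can play a Conversation and send Angie to a TargetPoint, optionally holding her until WaitDuration ends or Go releases her early.
; References are fetched on overlap because collisions can precede BeginPlay.
; One-shot cues destroy themselves after releasing Angie or being triggered by Derek.
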(event `self.ReceiveBeginPlay`)

(event `/Game/Monsters/Angie/Triggerable.Go`
  ;[1 1 1] If triggered by a conversation, it should release angie from waiting early.
  (set `self.preempted` true)
  (`/Game/Monsters/Angie/Angie.StopWaiting` (`self.angie`) :!label _label)
  ;[1 1 1] Delete self if it can only be activated once
  (if (`self.OneShot`) :!label _label_2
    (`self.K2_DestroyActor`)))

(event `self.ReceiveActorBeginOverlap`
  (params (OtherActor :type "Actor Object Reference"))
  ;[1 1 1] Because the first collisions happen before eventbeginplay
  (`|ExecutionSequence`
    (:`then_0`
      (set `self.Started` true)
      (bind _outactors (`GameplayStatics.GetAllActorsOfClass` "/Game/Monsters/Angie/Angie.Angie_C"))
      (set `self.angie` (`KismetArrayLibrary.Array_Get` _outactors))
      (bind _outactors_2 (`GameplayStatics.GetAllActorsOfClass` "/Game/Monsters/BlockingSmoke/BlockingSmoke_Blueprint.BlockingSmoke_Blueprint_C"))
      (set `self.Smoke` (`KismetArrayLibrary.Array_Get` _outactors_2)))
    (:`then_1`
      (if (== (`self.storyIndex`) (`/Game/Monsters/BlockingSmoke/BlockingSmoke_Blueprint.StoryIndex` (`self.Smoke`)))
        (`|ExecutionSequence`
          (:`then_0`
            ;[1 1 1] Stop angie if the trigger should and is triggered by her. Play conversations.
            (if (`self.TriggeredByAngie`)
              (bind _asangie (cast `/Game/Monsters/Angie/Angie` OtherActor))
              (if (`self.StopsAngie`)
                (`/Game/Monsters/Angie/Angie.StartWaiting` _asangie self)
                (`self.onEntered`)
                (`KismetSystemLibrary.Delay` (`self.WaitDuration`))
                (if (not (`self.preempted`))
                  (goto _label)))))
          (:`then_1`
            (if (`self.TriggeredByDerek`)
              (cast `/Game/Player/FirstPersonCharacter` OtherActor)
              (`self.onEntered`)
              (goto _label_2))))))))

(event `self.ReceiveTick`
  (params (DeltaSeconds :type "Float (single-precision)")))

(fn `onEntered`
  (`|ExecutionSequence`
    (:`then_0`
      (if (`KismetSystemLibrary.IsValid` (`self.Conversation`))
        (`/Game/Monsters/Angie/Conversation.Play` (`self.Conversation`))))
    (:`then_1`
      (if (`KismetSystemLibrary.IsValid` (`self.targetPoint`))
        (bind _asangie_controller (cast `/Game/Monsters/Angie/AngieController` (`Pawn.GetController` (`self.angie`))))
        (`/Game/Monsters/Angie/AngieController.SetDestination` _asangie_controller (`self.K2_GetActorLocation` (`self.targetPoint`)))))))

(fn `UserConstructionScript`)