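; Fire axe interactable object that presents itself to the player as an item to pick up.
; Highlight and UnHighlight toggle custom depth rendering on the Axe and Cube components to mark it visually.
; It exposes both components as interact colliders and returns an 'E' pick-up tooltip.
; The Blueprint holds no pickup logic of its own.
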(event `/Game/Blueprints/InteractableObjects/Interactable.Highlight`
  (`PrimitiveComponent.SetRenderCustomDepth` (`self.Axe`) true)
  (`PrimitiveComponent.SetRenderCustomDepth` (`self.Cube`) true))

(event `/Game/Blueprints/InteractableObjects/Interactable.UnHighlight`
  (`PrimitiveComponent.SetRenderCustomDepth` (`self.Axe`) false)
  (`PrimitiveComponent.SetRenderCustomDepth` (`self.Cube`) false))

(fn `GetInteractColliders`
  (returns (Collider :type "Array of ActorComponent Object Reference"))
  (return (`|MakeArray` (`self.Axe`) (`self.Cube`) :!type "ActorComponent Object Reference")))

(fn `GetTooltip`
  (returns (Tooltip :type Text))
  (return "'E' Pick up"))

(fn `UserConstructionScript`)