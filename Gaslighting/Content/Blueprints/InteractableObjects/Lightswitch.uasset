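; An interactable lightswitch that toggles the visibility of the lights in its Lights array.
; Interact alternates between playing and reversing a timeline that moves and rotates the Switch, with the lights toggling when the timeline finishes.
; Highlight and UnHighlight set custom depth rendering on the Backplate and Switch, which also serve as the interact colliders, and GetTooltip supplies the prompt text.
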(event `/Game/Blueprints/InteractableObjects/Interactable.Interact`
  (`/Engine/EditorBlueprintResources/StandardMacros.FlipFlop`
    (:`A`
      ;[1 1 1] Play switch animation
      (bind (_direction _rotationamount) (`Timeline|FlickSwitch` :!label _label)
        (:`Update`
          (`SceneComponent.K2_SetRelativeLocationAndRotation` (`self.Switch`) (`KismetMathLibrary.VLerp` (4.0 0.0 10.0) (4.0 0.0 -10.0) _rotationamount) (`KismetMathLibrary.RLerp` (struct :`Pitch` -30.0) (struct :`Pitch` 30.0) _rotationamount) false false))
        (:`Finished`
          ;[1 1 1] Toggle the lights on/off
          (for _array_element (`self.Lights`)
            (`SceneComponent.ToggleVisibility` (`Light.LightComponent` _array_element) false)))))
    (:`B`
      (goto _label :!via `Reverse`))))

(event `/Game/Blueprints/InteractableObjects/Interactable.Highlight`
  ;[1 1 1] Highlighting
  (`PrimitiveComponent.SetRenderCustomDepth` (`self.Backplate`) true)
  (`PrimitiveComponent.SetRenderCustomDepth` (`self.Switch`) true))

(event `/Game/Blueprints/InteractableObjects/Interactable.UnHighlight`
  ;[1 1 1] Highlighting
  (`PrimitiveComponent.SetRenderCustomDepth` (`self.Backplate`) false)
  (`PrimitiveComponent.SetRenderCustomDepth` (`self.Switch`) false))

(fn `GetInteractColliders`
  (returns (Collider :type "Array of ActorComponent Object Reference"))
  (return (`|MakeArray` (`self.Backplate`) (`self.Switch`) :!type "ActorComponent Object Reference")))

(fn `GetTooltip`
  (returns (Tooltip :type Text))
  (return "'E' Flip lightswitch"))

(fn `UserConstructionScript`)