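; Component that lets the player use nearby objects implementing Interactable and shows which one is being looked at.
; Interact and HighlightObject each line trace a short distance from the supplied camera against WorldDynamic objects.
; Highlighting enables custom depth on the hit actor's meshes and shows its tooltip in a widget created on BeginPlay.
; A missed trace clears the text and turns off the last hit actor's highlight.
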(event `Interact`
  (params (PlayerCam :type "CameraComponent Object Reference"))
  (bind _returnvalue (`SceneComponent.K2_GetComponentLocation` PlayerCam))
  ;[1 1 1] Interact with objects
  (bind (_outhit _returnvalue_2) (`KismetSystemLibrary.LineTraceSingleForObjects` _returnvalue (+ _returnvalue (* (`KismetMathLibrary.GetForwardVector` (`SceneComponent.K2_GetComponentRotation` PlayerCam)) 200.0)) (`|MakeArray` "ObjectTypeQuery2" :!type "EObjectTypeQuery Enum")))
  (if _returnvalue_2
    (bind _asinteractable (cast `/Game/Blueprints/InteractableObjects/Interactable` (`.HitActor` (`GameplayStatics.BreakHitResult` _outhit))))
    (`/Game/Blueprints/InteractableObjects/Interactable.Interact` _asinteractable)))

(event `HighlightObject`
  (params (PlayerCam :type "CameraComponent Object Reference"))
  (bind _returnvalue (`SceneComponent.K2_GetComponentLocation` PlayerCam))
  (bind _lasthit (`self.LastHit`))
  (bind _tooltips (`self.Tooltips`))
  (bind _returnvalue_2 (`Actor.K2_GetComponentsByClass` _lasthit "/Script/Engine.MeshComponent"))
  ;[1 1 1] Highlight interactable objects
  (bind (_outhit _returnvalue_3) (`KismetSystemLibrary.LineTraceSingleForObjects` _returnvalue (+ _returnvalue (* (`KismetMathLibrary.GetForwardVector` (`SceneComponent.K2_GetComponentRotation` PlayerCam)) 200.0)) (`|MakeArray` "ObjectTypeQuery2" :!type "EObjectTypeQuery Enum")))
  (if _returnvalue_3
    (bind _output_get (set `self.LastHit` (`.HitActor` (`GameplayStatics.BreakHitResult` _outhit))))
    (bind _asinteractable (cast `/Game/Blueprints/InteractableObjects/Interactable` _output_get))
    (bind _tooltip (`/Game/Blueprints/InteractableObjects/Interactable.GetTooltip` _asinteractable))
    (set `/Game/Blueprints/UI/Tooltips.Text` _tooltip _tooltips)
    (`/Engine/EditorBlueprintResources/StandardMacros.IsValid` _lasthit
      (:`Is Valid`
        (for _array_element _returnvalue_2
          (`PrimitiveComponent.SetRenderCustomDepth` _array_element true))))
    (else
      (set `/Game/Blueprints/UI/Tooltips.Text` "" _tooltips)
      (`/Engine/EditorBlueprintResources/StandardMacros.IsValid` _lasthit
        (:`Is Valid`
          (for _array_element_2 _returnvalue_2
            (`PrimitiveComponent.SetRenderCustomDepth` _array_element_2 false))
          (set `self.LastHit` null))))))

(event `self.ReceiveBeginPlay`
  ;[1 1 1] Set up tooltip UI
  (bind _returnvalue (`|CreateWidget` "/Game/Blueprints/UI/Tooltips.Tooltips_C"))
  (`UserWidget.AddToViewport` _returnvalue 0)
  (set `self.Tooltips` _returnvalue))