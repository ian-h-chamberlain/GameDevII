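; Interactable hinged door that the player opens and closes, with highlight and tooltip while active.
; Interacting plays or reverses a yaw timeline with knob and shut sounds, first stepping the player back if inside StepTrigger.
; Leaving InTrigger or OutTrigger while outside the other auto-closes the door after a short delay, optionally deactivating it through per-side lock flags.
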(event `/Game/Blueprints/InteractableObjects/Interactable.Interact`
  (bind _returnvalue (`GameplayStatics.GetPlayerCharacter` 0))
  ;[1 1 1] Step back if needed to open door
  (if (`self.IsActive`)
    (if (`self.IsOpen`)
      (set `self.IsOpen` false :!label _label)
      (bind (_direction _openness) (`Timeline|OpenAnim` :!via `Reverse` :!label _label_2)
        (:`Update`
          (`SceneComponent.K2_SetRelativeRotation` (`self.SM_Door`) (`KismetMathLibrary.MakeRotator` 0.0 0.0 _openness) false false))
        (:`DoorSound`
          ;[1 1 1] Comment
          (if (`|EnumEquality` _direction "Backward")
            (`AudioComponent.Play` (`self.Door_Shut`) 0.0)
            (else
              (`AudioComponent.Play` (`self.Knob_Turn`) 0.0)))))
      (else
        (if (`PrimitiveComponent.IsOverlappingActor` (`self.StepTrigger`) _returnvalue)
          (bind _asfirst_person_character (cast `/Game/FirstPersonBP/Blueprints/FirstPersonCharacter` _returnvalue))
          (`/Game/FirstPersonBP/Blueprints/FirstPersonCharacter.StepBack` _asfirst_person_character))
        (set `self.IsOpen` true)
        (goto _label_2)))))

(event `self.InTrigger.OnComponentEndOverlap`
  (params (OtherActor :type "Actor Object Reference") (OtherComp :type "PrimitiveComponent Object Reference") (OtherBodyIndex :type Integer))
  ;[1 1 1] Close door after walking through
  (cast `/Game/FirstPersonBP/Blueprints/FirstPersonCharacter` OtherActor)
  (if (not (`PrimitiveComponent.IsOverlappingActor` (`self.OutTrigger`) (`GameplayStatics.GetPlayerCharacter` 0)))
    (if (`self.LocksAfterIn`)
      (set `self.IsActive` false))
    (`KismetSystemLibrary.Delay` 0.2 :!label _label_3)
    (goto _label)))

(event `self.OutTrigger.OnComponentEndOverlap`
  (params (OtherActor :type "Actor Object Reference") (OtherComp :type "PrimitiveComponent Object Reference") (OtherBodyIndex :type Integer))
  ;[1 1 1] Close door after walking through
  (cast `/Game/FirstPersonBP/Blueprints/FirstPersonCharacter` OtherActor)
  (if (`PrimitiveComponent.IsOverlappingActor` (`self.InTrigger`) (`GameplayStatics.GetPlayerCharacter` 0))
    _
    (elif (`self.LocksAfterOut`)
      (set `self.IsActive` false)
      (goto _label_3)
      (else
        (goto _label_3)))))

(event `/Game/Blueprints/InteractableObjects/Interactable.Highlight`
  ;[1 1 1] Highlight this object
  (if (`self.IsActive`)
    (`PrimitiveComponent.SetRenderCustomDepth` (`self.SM_Door`) true)))

(event `/Game/Blueprints/InteractableObjects/Interactable.UnHighlight`
  ;[1 1 1] Highlight this object
  (`PrimitiveComponent.SetRenderCustomDepth` (`self.SM_Door`) false))

(fn `GetInteractColliders`
  (returns (Collider :type "Array of ActorComponent Object Reference"))
  (return (`|MakeArray` (`self.DoorCollider`) (`self.DoorFrameCollider`) :!type "ActorComponent Object Reference")))

(fn `GetTooltip`
  (returns (Tooltip :type Text))
  (if (`self.IsActive`)
    (return "'E' Open/close door")
    (else
      (return ""))))

(fn `UserConstructionScript`)