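; Interactable gas knob that the player turns, notifying listeners with the monsters it affects.
; Interact plays the GasKnob component and runs a Rotation timeline that adds a fixed yaw step on each update, then calls KnobTurn with MonstersAffected when finished.
; Highlighting toggles custom depth on both cube meshes, and the knob supplies its box collider and tooltip for interaction.
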(event `/Game/Blueprints/InteractableObjects/Interactable.Interact`
  ;[1 1 1] Comment
  (`AudioComponent.Play` (`self.Gas_Knob`) 0.0)
  (`Timeline|Rotation` :!via `PlayFromStart`
    (:`Update`
      (`self.K2_AddActorLocalRotation` (struct :`Pitch` 12.0)))
    (:`Finished`
      (`self.KnobTurn` (`self.MonstersAffected`)))))

(event `/Game/Blueprints/InteractableObjects/Interactable.Highlight`
  ;[1 1 1] Highlight / Unhighlight
  (`PrimitiveComponent.SetRenderCustomDepth` (`self.Cube`) true)
  (`PrimitiveComponent.SetRenderCustomDepth` (`self.Cube1`) true))

(event `/Game/Blueprints/InteractableObjects/Interactable.UnHighlight`
  ;[1 1 1] Highlight / Unhighlight
  (`PrimitiveComponent.SetRenderCustomDepth` (`self.Cube`) false)
  (`PrimitiveComponent.SetRenderCustomDepth` (`self.Cube1`) false))

(fn `GetInteractColliders`
  (returns (Collider :type "Array of ActorComponent Object Reference"))
  (return (`|MakeArray` (`self.Box`) :!type "ActorComponent Object Reference")))

(fn `GetTooltip`
  (returns (Tooltip :type Text))
  (return "'E' Turn knob"))

(fn `UserConstructionScript`)