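; PanicComponent tracks a panic meter that rises over time and signals a loss when it reaches the maximum.
; Tick adds PanicPerSecond scaled by delta time, clamps the level between zero and MaximumPanic, then prints a losing message once the cap is hit.
; AddPanic and RemovePanic adjust the level directly, with clamping applied only on the next Tick.
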(event `self.ReceiveBeginPlay`)

(event `self.ReceiveTick`
  (params (DeltaSeconds :type "Float (single-precision)"))
  (set `self.PanicLevel` (`KismetMathLibrary.FClamp` (+ (* (`self.PanicPerSecond`) DeltaSeconds) (`self.PanicLevel`)) 0.0 (`self.MaximumPanic`)))
  (if (>= (`self.PanicLevel`) (`self.MaximumPanic`))
    (`KismetSystemLibrary.PrintString` "oh no, you lost.")))

(fn `AddPanic`
  (params (Amount :type "Float (double-precision)"))
  (set `self.PanicLevel` (+ (`self.PanicLevel`) Amount)))

(fn `RemovePanic`
  (params (amount :type "Float (double-precision)"))
  (set `self.PanicLevel` (- (`self.PanicLevel`) amount)))